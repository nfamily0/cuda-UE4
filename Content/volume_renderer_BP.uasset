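; Volume renderer actor that displays a CUDA-rendered volume on its Plane mesh.
; BeginPlay calls ReadBighaed, then initializes CUDA rendering with the player camera transform, a fixed transfer range and two grey-to-white colors.
; Tick re-renders from the current camera.
; Both events feed the returned texture into the volume material's "volumeTexture" parameter, with Tick calling CreateDynamicMaterialInstance every frame rather than caching the instance.
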(event EventBeginPlay
  (Class|VolumeRenderer|ReadBighaed)
  (bind _returnvalue (Class|VolumeRenderer|CUDAVolumeRenderingInit (Variables|/Script/Engine.PlayerCameraManager|GetTransformComponent (Variables|/Script/Engine.PlayerController|GetPlayerCameraManager (Game|GetPlayerController 0))) "(X=100.000000,Y=140.000000)" "0.600000,0.600000,0.600000" "1.000000,1.000000,1.000000"))
  (bind _returnvalue_2 (Rendering|Material|CreateDynamicMaterialInstance (Variables|Default|GetPlane) 0 "/Game/VolumeMaterial.VolumeMaterial" "None" :!class /Script/Engine.PrimitiveComponent))
  (Rendering|Material|SetTextureParameterValue _returnvalue_2 "volumeTexture" _returnvalue))

(event EventTick
  (params (DeltaSeconds :type Float%20%28single-precision%29))
  (bind _returnvalue (Class|VolumeRenderer|CUDAVolumeRenderingTick (Variables|/Script/Engine.PlayerCameraManager|GetTransformComponent (Variables|/Script/Engine.PlayerController|GetPlayerCameraManager (Game|GetPlayerController 0))) "(X=100.000000,Y=140.000000)" "0.600000,0.600000,0.600000" "1.000000,1.000000,1.000000"))
  (bind _returnvalue_2 (Rendering|Material|CreateDynamicMaterialInstance (Variables|Default|GetPlane) 0 "/Game/VolumeMaterial.VolumeMaterial" "None" :!class /Script/Engine.PrimitiveComponent))
  (Rendering|Material|SetTextureParameterValue _returnvalue_2 "volumeTexture" _returnvalue))

(fn ConstructionScript)